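; Game mode for the Skvt game that handles respawning by moving a player into a surviving character.
; Respawn searches all BP_SkvtBaseChar actors for the first one still alive and has the given player controller possess it.
; When no living character remains, it casts the controller to BP_SkvtPlayerController and opens its menu instead.
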(event Custom|Respawn
  (params (PlayerController :type Controller%20Object%20Reference))
  (bind _newcharacter (CallFunction|FindValidCharacter))
  (Utilities|IsValid _newcharacter
    (:Is%20Valid
      (Pawn|Possess PlayerController _newcharacter))
    (:Is%20Not%20Valid
      (bind _asbp_skvt_player_controller (Utilities|Casting|CastToBP_SkvtPlayerController PlayerController))
      (Default|OpenMenu _asbp_skvt_player_controller))))

(fn ConstructionScript)

(fn FindValidCharacter
  (bind _outactors (Actor|GetAllActorsOfClass "/Game/Skvt/Characters/BP_SkvtBaseChar.BP_SkvtBaseChar_C"))
  (for _array_element _outactors
    (if (Default|IsAlive _array_element)
      (return _array_element)))
  (return 0))