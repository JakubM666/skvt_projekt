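; Base NPC character Blueprint that handles taking damage and dying.
; Any damage passes to the health component for processing and plays a punch hit-reaction montage.
; When the health component signals death, the mesh switches to physics simulation, movement is disabled, and the actor is destroyed after a short timer.
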(event OnDeath(SkvtHeatlhComponent)
  (Physics|SetSimulatePhysics (Variables|Character|GetMesh) true)
  (Pawn|Components|CharacterMovement|DisableMovement (Variables|Character|GetCharacterMovement))
  (Utilities|Time|SetTimerbyEvent (delegate Custom|FinalizeDeath) 2.0))

(event Custom|FinalizeDeath
  (Actor|DestroyActor))

(event EventBeginPlay
  (|CallParentFunction) ; This node is disabled and will not be called.\nDrag off pins to build functionality.
)

(event Collision|EventActorBeginOverlap
  (params (OtherActor :type Actor%20Object%20Reference))
  (|CallParentFunction OtherActor) ; This node is disabled and will not be called.\nDrag off pins to build functionality.
)

(event EventTick
  (params (DeltaSeconds :type Float%20%28single-precision%29))
  (|CallParentFunction DeltaSeconds) ; This node is disabled and will not be called.\nDrag off pins to build functionality.
)

(event Game|Damage|EventAnyDamage
  (params (Damage :type Float%20%28single-precision%29) (DamageType :type Damage%20Type%20Object%20Reference) (InstigatedBy :type Controller%20Object%20Reference) (DamageCauser :type Actor%20Object%20Reference))
  (Default|ProcessDamage (Variables|Default|GetSkvtHeatlhComponent) Damage)
  (Animation|PlayAnimMontage "/Game/Skvt/Characters/Animations/Attacks/AM_Hit_punch.AM_Hit_punch" 1.0 "None"))

(fn ConstructionScript
  (|CallParentFunction))