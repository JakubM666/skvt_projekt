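; Player controller for the Skvt game that owns the UI and lets the player swap between male and female characters.
; BeginPlay spawns the HUD and adds the default and swap-pawn Enhanced Input mapping contexts.
; The menu input toggles a main menu that pauses the game and shows the cursor, with a similar game-finished screen and a pass-through for health bar updates.
; Swap input possesses the first found actor of the other character class.
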(event Input|EnhancedActionEvents|EnhancedInputActionIA_Swap
  (params (ActionValue :type Boolean) (ElapsedSeconds :type Float%20%28double-precision%29) (TriggeredSeconds :type Float%20%28double-precision%29) (InputAction :type Input%20Action%20Object%20Reference :default "/Game/Skvt/Characters/Input/Actions/IA_Swap.IA_Swap"))
  (:Triggered
    (if (.bSuccess (Utilities|Casting|CastToBP_SkvtCharacterMale (Game|Player|GetPlayerPawn 0)))
      (bind _returnvalue (Actor|GetActorOfClass "/Game/Skvt/Characters/BP_SkvtCharacterFemale.BP_SkvtCharacterFemale_C"))
      (Pawn|Possess _returnvalue)
      (else
        (bind _returnvalue_2 (Actor|GetActorOfClass "/Game/Skvt/Characters/BP_SkvtCharacterMale.BP_SkvtCharacterMale_C"))
        (Pawn|Possess _returnvalue_2)))))

(event Input|EnhancedActionEvents|EnhancedInputActionIA_OpenMenu
  (params (ActionValue :type Boolean) (ElapsedSeconds :type Float%20%28double-precision%29) (TriggeredSeconds :type Float%20%28double-precision%29) (InputAction :type Input%20Action%20Object%20Reference :default "/Game/Skvt/Characters/Input/Actions/IA_OpenMenu.IA_OpenMenu"))
  (:Triggered
    (if (CallFunction|IsMenuOpen)
      (CallFunction|CloseMenu)
      (else
        (CallFunction|OpenMenu)))))

(event EventBeginPlay
  (bind _self self)
  (bind _returnvalue (PlayerController|LocalPlayerSubsystems|GetEnhancedInputLocalPlayerSubsystem _self))
  (CallFunction|SpawnHUD)
  (Utilities|IsValid _returnvalue
    (:Is%20Valid
      (Input|AddMappingContext _returnvalue "/Game/ThirdPerson/Input/IMC_Default.IMC_Default" 0 "(bIgnoreAllPressedKeysUntilRelease=True,bForceImmediately=False)")
      (Input|AddMappingContext _returnvalue "/Game/Skvt/Characters/Input/IMC_SwapPawn.IMC_SwapPawn" 0 "(bIgnoreAllPressedKeysUntilRelease=True,bForceImmediately=False)"))))

(fn ConstructionScript)

(fn OpenMenu
  (bind _returnvalue (UserInterface|CreateWidget "/Game/Skvt/UI/Widgets/Menu/WBP_MainMenu.WBP_MainMenu_C" self))
  (bind _output_get (Variables|Default|SetMainMenuRef _returnvalue))
  (UserInterface|Viewport|AddtoViewport _output_get 0)
  (Variables|Default|SetbShowMouseCursor true)
  (Input|SetInputModeGameandUI self 0 "DoNotLock" true false)
  (Game|SetGamePaused true))

(fn CloseMenu
  (Widget|RemovefromParent (Variables|Default|GetMainMenuRef))
  (Variables|Default|SetMainMenuRef 0)
  (Input|SetInputModeGameOnly self false)
  (Variables|Default|SetbShowMouseCursor false)
  (Game|SetGamePaused false))

(fn IsMenuOpen
  (return (Utilities|IsValid (Variables|Default|GetMainMenuRef))))

(fn SpawnHUD
  (bind _returnvalue (UserInterface|CreateWidget "/Game/Skvt/UI/Widgets/HUD/WBP_HUD.WBP_HUD_C" self))
  (bind _output_get (Variables|Default|SetHudRef _returnvalue))
  (UserInterface|Viewport|AddtoViewport _output_get 0))

(fn UpdateHealthBar
  (params (NewHealthBar :type Skvt%20Heatlh%20Component%20Object%20Reference))
  (Default|InitializeHealthBar (Variables|Default|GetHudRef) NewHealthBar))

(fn OpenGameFinishedMenu
  (bind _returnvalue (UserInterface|CreateWidget "/Game/Skvt/UI/Widgets/Menu/WBP_GameFinished.WBP_GameFinished_C" self))
  (bind _output_get (Variables|Default|SetGameFinishedMenuRef _returnvalue))
  (UserInterface|Viewport|AddtoViewport _output_get 0)
  (Variables|Default|SetbShowMouseCursor true)
  (Input|SetInputModeGameandUI self 0 "DoNotLock" true false)
  (Game|SetGamePaused true))