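; BP_WallSconce is a configurable spot-light wall sconce that can be toggled and marked as EMPed.
; InitLight applies brightness, color, cone angles and on/off visibility at construction and BeginPlay, while ToggleLight updates visibility.
; EMPed stores its flag and activates the spark effect regardless of value, without changing the light.
; Tick runs a sphere overlap for BP_SkvtBaseChar, drawing a green or red debug sphere to show the result.
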(event EventBeginPlay
  (CallFunction|InitLight))

(event EventTick
  (params (DeltaSeconds :type Float%20%28single-precision%29))
  (bind _returnvalue (Transformation|GetActorLocation))
  (bind _returnvalue_2 (Collision|SphereOverlapActors _returnvalue 2.8e+02 (Variables|Default|GetSomething) "/Game/Skvt/Characters/BP_SkvtBaseChar.BP_SkvtBaseChar_C"))
  (if _returnvalue_2
    (Rendering|Debug|DrawDebugSphere _returnvalue 3e+01 12 "(R=0.053151,G=1.000000,B=0.000000,A=1.000000)" 0.0 1.0)
    (else
      (Rendering|Debug|DrawDebugSphere _returnvalue 3e+01 12 "(R=1.000000,G=0.018187,B=0.000000,A=1.000000)" 0.0 1.0))))

(fn ConstructionScript
  (CallFunction|InitLight))

(fn InitLight
  (bind _sconcelight (Variables|Default|GetSconceLight))
  (Rendering|Components|Light|SetIntensity _sconcelight (Variables|Light|GetBrightness))
  (Rendering|Components|Light|SetLightColor _sconcelight (Variables|Light|GetColor) true)
  (Rendering|Lighting|SetInnerConeAngle _sconcelight (Variables|Light|GetInner%20Cone%20Angle))
  (Rendering|Lighting|SetOuterConeAngle _sconcelight (Variables|Light|GetOuter%20Cone%20Angle))
  (Rendering|SetVisibility (Variables|Default|GetSconceLight) (Variables|Default|GetIsOn) false))

(fn ToggleLight
  (params (isOn :type Boolean))
  (bind _output_get (Variables|Default|SetIsOn isOn))
  (Rendering|SetVisibility (Variables|Default|GetSconceLight) _output_get false))

(fn EMPed
  (params (EMPed :type Boolean))
  (Variables|Default|SetEMPed? EMPed)
  (Components|Activation|Activate (Variables|Default|GetP_Sparks) false))